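; Security monitor Blueprint that shows the live feed of linked camera actors on its screen mesh.
; On BeginPlay it applies a dynamic material with set brightness, fed by a render target on the first camera's scene capture, sized from viewport and camera quality.
; swapcamra detaches the current capture and cycles to the next camera with a newly created render target.
; newplayerinput forwards horizontal and vertical input to rotate the active camera.
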(event Custom|swapcamra
  (bind _returnvalue (Viewport|GetViewportSize))
  (Variables|/Script/Engine.SceneCaptureComponent2D|SetTextureTarget (Variables|/Game/cam_screen/cemra1.cemra1_C|GetSceneCaptureComponent2D (Utilities|Array|Get(acopy) (Variables|Default|Getlinkedcam) (Variables|Default|Getcurentcamra))) 0)
  (Math|Integer|IncrementInt (Variables|Default|Getcurentcamra)
    (:%20%20
      (if (>= (Variables|Default|Getcurentcamra) (Utilities|Array|Length (Variables|Default|Getlinkedcam)))
        (Variables|Default|Setcurentcamra 0))
      (bind _returnvalue_2 (Rendering|CreateRenderTarget2D (Math|Float|Truncate (* (.x _returnvalue) (Variables|/Game/cam_screen/cemra1.cemra1_C|Getcameraqualitylevel (Utilities|Array|Get(acopy) (Variables|Default|Getlinkedcam) (Variables|Default|Getcurentcamra))))) (Math|Float|Truncate (* (.y _returnvalue) (Variables|/Game/cam_screen/cemra1.cemra1_C|Getcameraqualitylevel (Utilities|Array|Get(acopy) (Variables|Default|Getlinkedcam) (Variables|Default|Getcurentcamra))))) "RTF_RGBA16f"))
      (bind _output_get (Variables|Default|Setcamra_rt _returnvalue_2))
      (bind _output_get_2 (Variables|/Script/Engine.SceneCaptureComponent2D|SetTextureTarget (Variables|/Game/cam_screen/cemra1.cemra1_C|GetSceneCaptureComponent2D (Utilities|Array|Get(acopy) (Variables|Default|Getlinkedcam) (Variables|Default|Getcurentcamra))) _output_get))
      (Rendering|Material|SetTextureParameterValue (Variables|Default|Getcamra_mat) "texture" _output_get_2))))

(event Custom|newplayerinput
  (params (Horizentalvalue :type Float%20%28double-precision%29) (Verticalvelue :type Float%20%28double-precision%29))
  (Default|Rotatecamera (Utilities|Array|Get(acopy) (Variables|Default|Getlinkedcam) (Variables|Default|Getcurentcamra)) Horizentalvalue Verticalvelue))

(event EventBeginPlay
  (bind _returnvalue (Viewport|GetViewportSize))
  (bind _linkedcam (Variables|Default|Getlinkedcam))
  (bind _output (Utilities|Array|Get(acopy) _linkedcam))
  (bind _cameraqualitylevel (Variables|/Game/cam_screen/cemra1.cemra1_C|Getcameraqualitylevel _output))
  (Utilities|IsValid (Utilities|Array|Get(acopy) (Variables|Default|Getlinkedcam))
    (:Is%20Valid
      (bind _returnvalue_2 (Rendering|Material|CreateDynamicMaterialInstance "/Game/cam_screen/cemra_mat.cemra_mat" "None" "None" :!class /Script/Engine.KismetMaterialLibrary))
      (bind _output_get (Variables|Default|Setcamra_mat _returnvalue_2))
      (Rendering|Material|SetMaterial (Variables|Default|Getmonitor) 0 _output_get)
      (bind _returnvalue_3 (Rendering|CreateRenderTarget2D (Math|Float|Truncate (* (.x _returnvalue) _cameraqualitylevel)) (Math|Float|Truncate (* (.y _returnvalue) _cameraqualitylevel)) "RTF_RGBA16f"))
      (bind _output_get_2 (Variables|Default|Setcamra_rt _returnvalue_3))
      (bind _output_get_3 (Variables|/Script/Engine.SceneCaptureComponent2D|SetTextureTarget (Variables|/Game/cam_screen/cemra1.cemra1_C|GetSceneCaptureComponent2D (Utilities|Array|Get(acopy) (Variables|Default|Getlinkedcam))) _output_get_2))
      (Rendering|Material|SetTextureParameterValue (Variables|Default|Getcamra_mat) "texture" _output_get_3)
      (Rendering|Material|SetScalarParameterValue (Variables|Default|Getcamra_mat) "screenbrightness" (Variables|Default|Getscreenbrightness) :!class /Script/Engine.MaterialInstanceDynamic))))

(fn ConstructionScript)