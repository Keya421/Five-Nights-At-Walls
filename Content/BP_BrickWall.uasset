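; BP_BrickWall is a roaming jumpscare threat that advances through six rooms toward an attack on the player.
; A looping timer randomly steps it along an array of room actors.
; At the last room it waits, then either moves to world origin if Door 1 is closed or plays a bark, shows a jumpscare widget and quits the game.
; Older per-room random-move events remain, but their timers are disconnected.
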(event Custom|TIme
  (if (Math|Random|RandomBool)
    (bind _result (Math|Integer|IncrementInt (Variables|Default|GetRoomCounter))
      (:%20%20
        (bind _output_get (Variables|Default|SetSelectedLocation (Utilities|Array|Get(acopy) (Variables|Default|GetLocationArray) _result)))
        (Transformation|SetActorLocation (Transformation|GetActorLocation _output_get) false false)
        (if (== (Variables|Default|GetRoomCounter) 5)
          (Development|PrintString "Wall is in room 6")
          (Utilities|FlowControl|Delay 5.0)
          (bind _asbp_first_person_character (Utilities|Casting|CastToBP_FirstPersonCharacter (Game|GetPlayerCharacter 0)))
          (if (Variables|/Game/FirstPerson/Blueprints/BP_FirstPersonCharacter.BP_FirstPersonCharacter_C|GetisDoor1Closed _asbp_first_person_character)
            (Transformation|SetActorLocation "0, 0, 0" false false)
            (else
              (Audio|PlaySound2D "/Game/Door/bark.bark" 3.0 1.0 0.2 0 0)
              (bind _returnvalue (UserInterface|CreateWidget "/Game/jumpscarewall.jumpscarewall_C"))
              (UserInterface|Viewport|AddtoViewport _returnvalue 0)
              (Utilities|FlowControl|Delay 2.0)
              (Game|QuitGame 0 "Quit" false))))))))

(event Custom|room2
  (bind _room2ref (Variables|Default|GetRoom2Ref))
  (bind _cube (Variables|/Game/Room1.Room1_C|GetCube _room2ref))
  (bind _returnvalue (Transformation|GetWorldLocation _cube))
  (if (Math|Random|RandomBool)
    (if (and (Math|Random|RandomBool) (Variables|Default|GetisInRoom1\))
      (Transformation|SetActorLocation (Math|Vector|MakeVector (.x _returnvalue) (.y _returnvalue) (.z _returnvalue)) false false)
      (Variables|Default|SetisInRoom1\ false)
      (Variables|Default|SetisInroom2 true)
      (Variables|Default|Setisinroom3 false)
      (Variables|Default|Setisinroom4 false)
      (Variables|Default|Setisinroom5 false)
      (Variables|Default|Setisinroom6 false))))

(event Custom|room333
  (bind _room3 (Variables|Default|Getroom3))
  (bind _cube (Variables|/Game/Room1.Room1_C|GetCube _room3))
  (bind _returnvalue (Transformation|GetWorldLocation _cube))
  (if (Math|Random|RandomBool)
    (if (and (Math|Random|RandomBool) (Variables|Default|GetisInroom2))
      (Transformation|SetActorLocation (Math|Vector|MakeVector (.x _returnvalue) (.y _returnvalue) (.z _returnvalue)) false false)
      (Variables|Default|SetisInRoom1\ false)
      (Variables|Default|SetisInroom2 false)
      (Variables|Default|Setisinroom3 true)
      (Variables|Default|Setisinroom4 false)
      (Variables|Default|Setisinroom5 false)
      (Variables|Default|Setisinroom6 false))))

(event Custom|roon4
  (bind _room4 (Variables|Default|Getroom4))
  (bind _cube (Variables|/Game/Room1.Room1_C|GetCube _room4))
  (bind _returnvalue (Transformation|GetWorldLocation _cube))
  (if (Math|Random|RandomBool)
    (if (and (Math|Random|RandomBool) (Variables|Default|Getisinroom3))
      (Transformation|SetActorLocation (Math|Vector|MakeVector (.x _returnvalue) (.y _returnvalue) (.z _returnvalue)) false false)
      (Variables|Default|SetisInRoom1\ false)
      (Variables|Default|SetisInroom2 false)
      (Variables|Default|Setisinroom3 false)
      (Variables|Default|Setisinroom4 true)
      (Variables|Default|Setisinroom5 false)
      (Variables|Default|Setisinroom6 false))))

(event Custom|room55
  (bind _room5 (Variables|Default|Getroom5))
  (bind _cube (Variables|/Game/Room1.Room1_C|GetCube _room5))
  (bind _returnvalue (Transformation|GetWorldLocation _cube))
  (if (Math|Random|RandomBool)
    (if (and (Math|Random|RandomBool) (Variables|Default|Getisinroom4))
      (Transformation|SetActorLocation (Math|Vector|MakeVector (.x _returnvalue) (.y _returnvalue) (.z _returnvalue)) false false)
      (Variables|Default|SetisInRoom1\ false)
      (Variables|Default|SetisInroom2 false)
      (Variables|Default|Setisinroom3 false)
      (Variables|Default|Setisinroom4 false)
      (Variables|Default|Setisinroom5 true)
      (Variables|Default|Setisinroom6 false))))

(event Custom|room66
  (bind _room6 (Variables|Default|Getroom6))
  (bind _cube (Variables|/Game/Room1.Room1_C|GetCube _room6))
  (bind _returnvalue (Transformation|GetWorldLocation _cube))
  (if (Math|Random|RandomBool)
    (if (and (Math|Random|RandomBool) (Variables|Default|Getisinroom5))
      (Transformation|SetActorLocation (Math|Vector|MakeVector (.x _returnvalue) (.y _returnvalue) (.z _returnvalue)) false false)
      (Variables|Default|SetisInRoom1\ false)
      (Variables|Default|SetisInroom2 false)
      (Variables|Default|Setisinroom3 false)
      (Variables|Default|Setisinroom4 false)
      (Variables|Default|Setisinroom5 false)
      (Variables|Default|Setisinroom6 true))))

(event EventBeginPlay
  (Utilities|Time|SetTimerbyEvent (delegate Custom|TIme) 4.0 true)
  (Variables|Default|SetLocationArray (Utilities|Array|MakeArray (Variables|Default|GetRoom1Ref) (Variables|Default|GetRoom2Ref) (Variables|Default|Getroom3) (Variables|Default|Getroom4) (Variables|Default|Getroom5) (Variables|Default|Getroom6))))

(event Collision|EventActorBeginOverlap
  (params (OtherActor :type Actor%20Object%20Reference)))

(event EventTick
  (params (DeltaSeconds :type Float%20%28single-precision%29)))

(fn ConstructionScript)